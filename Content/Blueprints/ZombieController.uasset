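; ZombieController places zombies at the player's cursor in the village defense game.
; When OnSetDestinationPressed fires, it checks that the game mode's resource store still holds zombies.
; It then spawns a ZombieBP slightly above the pawn's CursorToWorld location, regardless of collision, and deducts one zombie from the store.
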(event EventBeginPlay)

(event EventTick
  (params (DeltaSeconds :type Float%20%28single-precision%29)))

(event EventOnSetDestinationPressed
  (bind _asvillage_defense_game_mode (Utilities|Casting|CastToVillageDefenseGameMode (Game|GetGameMode)))
  (if (> (Class|ResourceStore|GetZombies (Class|GGJ18GameModeBase|GetResourceStore _asvillage_defense_game_mode)) 0)
    (bind _asmy_default_pawn (Utilities|Casting|CastToMyDefaultPawn (Game|Player|GetPlayerPawn 0)))
    (Game|SpawnActorfromClass "/Game/Blueprints/Pawns/ZombieBP.ZombieBP_C" (Math|Transform|MakeTransform (+ (Transformation|GetWorldLocation (Variables|/Script/GGJ18.MyDefaultPawn|GetCursorToWorld _asmy_default_pawn)) "0, 0,108.062599") "0, 0, 0" "1,1,1") "AlwaysSpawn" 0 0)
    (Class|ResourceStore|LoseZombies (Class|GGJ18GameModeBase|GetResourceStore _asvillage_defense_game_mode) 1)))

(fn ConstructionScript)